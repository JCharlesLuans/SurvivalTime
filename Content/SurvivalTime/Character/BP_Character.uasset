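; Player character for a block-placing game, with movement, jump and mouse look, that adds the master HUD to the viewport on BeginPlay.
; Shortcut inputs set NumeroRaccourci, which serves as the block ID to place.
; The Casser input line-traces from the camera and, on hitting BP_Map, passes the impact point and ID through S_PlacerBloc to M_PlacerBloc (apparently a server-to-multicast chain), which calls the map's Placer.
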(event `self.ReceiveBeginPlay`
  (bind _returnvalue (`|CreateWidget` "/Game/SurvivalTime/UI/BPW__MasterHUD.BPW__MasterHUD_C"))
  (`UserWidget.AddToViewport` _returnvalue 0))

(event `InputAxis|Vertical`
  (params (AxisValue :type "Float (single-precision)"))
  ;[1 1 1] Déplaement
  ;;[1 1 1] Déplacement sur avant / arriere
  (`self.AddMovementInput` (`self.GetActorForwardVector`) AxisValue))

(event `InputAction|Jump`
  (params (Key :type "Key Structure"))
  ;[1 1 1] Déplaement
  ;;[1 1 1] Saut
  (:`Pressed`
    (`self.Jump`)))

(event `InputAction|Raccourci1`
  (params (Key :type "Key Structure"))
  (:`Pressed`
    (bind _output_get (set `self.numeroRaccourci` 0))
    (`KismetSystemLibrary.PrintString` (`KismetStringLibrary.Conv_IntToString` _output_get))))

(event `InputAction|Raccourci2`
  (params (Key :type "Key Structure"))
  (:`Pressed`
    (bind _output_get (set `self.numeroRaccourci` 1))
    (`KismetSystemLibrary.PrintString` (`KismetStringLibrary.Conv_IntToString` _output_get))))

(event `InputAxis|Horizontal`
  (params (AxisValue :type "Float (single-precision)"))
  ;[1 1 1] Déplaement
  ;;[1 1 1] Déplacement droite gauche
  (`self.AddMovementInput` (`self.GetActorRightVector`) AxisValue))

(event `InputAction|Raccourci3`
  (params (Key :type "Key Structure"))
  (:`Pressed`
    (bind _output_get (set `self.numeroRaccourci` 2))
    (`KismetSystemLibrary.PrintString` (`KismetStringLibrary.Conv_IntToString` _output_get))))

(event `InputAxis|Turn`
  (params (AxisValue :type "Float (single-precision)"))
  ;[1 1 1] Rotation personnage
  (`self.AddControllerYawInput` AxisValue))

(event `InputAxis|LookUp`
  (params (AxisValue :type "Float (single-precision)"))
  ;[1 1 1] Rotation camera
  (`self.AddControllerPitchInput` AxisValue))

(event `InputAction|Casser`
  (params (Key :type "Key Structure"))
  (bind _camera (`self.Camera`))
  (bind _returnvalue (`SceneComponent.K2_GetComponentLocation` _camera))
  ;[1 1 1] Plaçage de bloc
  (:`Pressed`
    (bind _outhit (`KismetSystemLibrary.LineTraceSingle` _returnvalue (+ _returnvalue (* (`SceneComponent.GetForwardVector` _camera) 1000.0)) "TraceTypeQuery1"))
    (bind (_bblockinghit _binitialoverlap _time _distance _location _impactpoint _normal _impactnormal _physmat _hitactor) (`GameplayStatics.BreakHitResult` _outhit))
    (bind _asbp_map (cast `/Game/SurvivalTime/Blueprint/BP_Map` _hitactor))
    (`self.S_PlacerBloc` _asbp_map _impactpoint (`self.numeroRaccourci`))))

(event `S_PlacerBloc`
  (params (Map :type "/Game/SurvivalTime/Blueprint/BP_Map Object Reference") (Position :type "Vector Structure") (`Id Bloc` :type Integer))
  ;[1 1 1] Plaçage de bloc
  (`self.M_PlacerBloc` Position Map `Id Bloc`))

(event `M_PlacerBloc`
  (params (Position :type "Vector Structure") (Map :type "/Game/SurvivalTime/Blueprint/BP_Map Object Reference") (idBloc :type Integer))
  ;[1 1 1] Plaçage de bloc
  (`/Game/SurvivalTime/Blueprint/BP_Map.Placer` Map Position idBloc))

(fn `UserConstructionScript`)