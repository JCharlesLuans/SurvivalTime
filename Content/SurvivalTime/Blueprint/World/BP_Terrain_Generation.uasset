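; Voxel terrain actor that builds a block world of grass (Herbe), dirt (Terre) and stone (Pierre) through instanced mesh components.
; Construction script runs GenerationMonde, offsetting each column by three summed sine-product waves.
; Stone sits beneath dirt, with grass topping only columns above the SolTerre threshold.
; Placer chains through S_/M_ events to add a grid-snapped block by ID; Casser (break) chains likewise but ends in an empty event.
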(event `Placer`
  (params (Position :type "Vector Structure") (`Id bloc` :type Integer))
  ;[1 1 1] Placage de bloc sur la map
  (`self.S_Placer` Position `Id bloc`))

(event `S_Placer`
  (params (Position :type "Vector Structure") (idBloc :type Integer))
  ;[1 1 1] Placage de bloc sur la map
  (`self.M_PlacerBloc` Position idBloc))

(event `M_PlacerBloc`
  (params (Position :type "Vector Structure") (idBloc :type Integer))
  (bind _returnvalue (`KismetMathLibrary.Conv_IntToDouble` (`self.taille tuile`)))
  (bind _returnvalue_2 (select `int` (`self.id bloc`) :`0` (`self.Herbe`) :`1` (`self.Terre`) :`2` (`self.Pierre`)))
  ;[1 1 1] Placage de bloc sur la map
  (set `self.id bloc` idBloc)
  (`/Engine/EditorBlueprintResources/StandardMacros.IsValid` _returnvalue_2
    (:`Is Valid`
      (`InstancedStaticMeshComponent.AddInstance` _returnvalue_2 (`KismetMathLibrary.MakeTransform` (`KismetMathLibrary.MakeVector` (`KismetMathLibrary.GridSnap_Float` (.x Position) _returnvalue) (`KismetMathLibrary.GridSnap_Float` (.y Position) _returnvalue) (`KismetMathLibrary.GridSnap_Float` (.z Position) _returnvalue)))))))

(event `Casser`
  (params (Position :type "Vector Structure"))
  (`self.S_Casser` Position))

(event `S_Casser`
  (params (Position :type "Vector Structure"))
  (`self.M_Casser` Position))

(event `M_Casser`
  (params (Position :type "Vector Structure")))

(fn `GenerationMonde`
  (locals (`index longueur` :type Integer) (`index largeur` :type Integer) (`index hauteur` :type Integer) (`sol terre` :type Integer))
  (bind _frequance1 (`self.frequance1`))
  (bind _frequance2 (`self.frequance2`))
  (bind _frequance3 (`self.frequance3`))
  (bind _taille_tuile (`self.taille tuile`))
  (bind _returnvalue (`KismetMathLibrary.Conv_IntToDouble` (+ (* _taille_tuile (`local.index hauteur`)) (* (`KismetMathLibrary.FFloor` (+ (* (`KismetMathLibrary.DegSin` (* (`local.index longueur`) _frequance1)) (`KismetMathLibrary.DegSin` (* (`local.index largeur`) _frequance1)) (`self.hauteur1`)) (* (`KismetMathLibrary.DegSin` (* (* (`local.index longueur`) _frequance2) 0.7)) (`KismetMathLibrary.DegSin` (* (`local.index largeur`) _frequance2)) (`self.hauteur2`)) (* (`KismetMathLibrary.DegSin` (* (`local.index longueur`) _frequance3)) (`KismetMathLibrary.DegSin` (* (* (`local.index largeur`) _frequance3) 0.4)) (`self.hauteur3`)))) (`self.taille tuile`)))))
  (bind _returnvalue_2 (`KismetMathLibrary.MakeVector` (`KismetMathLibrary.Conv_IntToDouble` (* (`local.index longueur`) _taille_tuile)) (`KismetMathLibrary.Conv_IntToDouble` (* _taille_tuile (`local.index largeur`))) _returnvalue))
  (bind _returnvalue_3 (`KismetMathLibrary.Conv_VectorToTransform` _returnvalue_2))
  (bind _returnvalue_4 (`KismetMathLibrary.Conv_VectorToTransform` _returnvalue_2))
  (for _index (range 1 (+ (`self.longueur`) 1))
    (set `local.index longueur` _index)
    (for _index_2 (range 1 (+ (`self.largeur`) 1))
      (set `local.index largeur` _index_2)
      (for _index_3 (range 1 (+ (`self.hauteur`) 1))
        (bind _output_get (set `local.index hauteur` _index_3))
        (if (== _output_get (`self.hauteur`))
          (if (> _returnvalue (`KismetMathLibrary.Conv_IntToDouble` (* (`self.taille tuile`) (+ (`local.sol terre`) (`self.hauteur`)))))
            (`InstancedStaticMeshComponent.AddInstance` (`self.Herbe`) _returnvalue_3)
            (else
              (`InstancedStaticMeshComponent.AddInstance` (`self.Terre`) _returnvalue_3)))
          (elif (> (`local.index hauteur`) (- (`self.hauteur`) 3))
            (`InstancedStaticMeshComponent.AddInstance` (`self.Terre`) _returnvalue_4)
            (else
              (`InstancedStaticMeshComponent.AddInstance` (`self.Pierre`) _returnvalue_4))))))))

(fn `UserConstructionScript`
  (`self.GenerationMonde`))