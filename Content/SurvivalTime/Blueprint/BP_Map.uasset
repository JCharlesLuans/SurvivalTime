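; BP_Map is the voxel world actor that generates block terrain on BeginPlay and handles block placement.
; GenerationMonde sums three sine-product layers into grid heights, adding Herbe (grass) instances above zero and Terre (dirt) otherwise.
; The column fill beneath the surface with dirt and Pierre (stone) is unwired, so only the surface spawns.
; Placer chains through S_Placer to M_PlacerBloc, which adds a grid-snapped Pierre instance.
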(event `self.ReceiveBeginPlay`
  (`self.GenerationMonde`))

(event `Placer`
  (params (Position :type "Vector Structure"))
  (`self.S_Placer` Position))

(event `S_Placer`
  (params (Position :type "Vector Structure"))
  (`self.M_PlacerBloc` Position))

(event `M_PlacerBloc`
  (params (Position :type "Vector Structure"))
  (bind _returnvalue (`KismetMathLibrary.Conv_IntToDouble` (`self.taille tuile`)))
  (`KismetSystemLibrary.PrintString` "M_Placer a bien ete appeller")
  (`InstancedStaticMeshComponent.AddInstance` (`self.Pierre`) (`KismetMathLibrary.MakeTransform` (`KismetMathLibrary.MakeVector` (`KismetMathLibrary.GridSnap_Float` (.x Position) _returnvalue) (`KismetMathLibrary.GridSnap_Float` (.y Position) _returnvalue) (`KismetMathLibrary.GridSnap_Float` (.z Position) _returnvalue))))
  (`KismetSystemLibrary.PrintString` "BP_Map; Bloc placer"))

(fn `GenerationMonde`
  (bind _frequance1 (`self.frequance1`))
  (bind _frequance2 (`self.frequance2`))
  (bind _frequance3 (`self.frequance3`))
  (bind _taille_tuile (`self.taille tuile`))
  (bind _returnvalue (* (`KismetMathLibrary.Round` (`KismetMathLibrary.Conv_IntToDouble` (+ (`self.nombreCouche`) (`KismetMathLibrary.FTrunc` (+ (* (`KismetMathLibrary.DegSin` (* (`self.index longueur`) _frequance1)) (`KismetMathLibrary.DegSin` (* (`self.index largeur`) _frequance1)) (`self.hauteur1`)) (* (`KismetMathLibrary.DegSin` (* (* (`self.index longueur`) _frequance2) 0.7)) (`KismetMathLibrary.DegSin` (* (`self.index largeur`) _frequance2)) (`self.hauteur2`)) (* (`KismetMathLibrary.DegSin` (* (`self.index longueur`) _frequance3)) (`KismetMathLibrary.DegSin` (* (* (`self.index largeur`) _frequance3) 0.4)) (`self.hauteur3`))))))) (`self.taille tuile`)))
  (bind _returnvalue_2 (`KismetMathLibrary.Conv_IntToDouble` _returnvalue))
  (for _index (range 1 (+ (`self.longueur`) 1))
    (set `self.index longueur` _index)
    (for _index_2 (range 1 (+ (`self.largeur`) 1))
      (set `self.index largeur` _index_2)
      (bind _output_get (set `self.vector` (`KismetMathLibrary.MakeVector` (`KismetMathLibrary.Conv_IntToDouble` (* (`self.index longueur`) _taille_tuile)) (`KismetMathLibrary.Conv_IntToDouble` (* _taille_tuile (`self.index largeur`))) _returnvalue_2)))
      (set `self.index hauteur` _returnvalue)
      (if (> _returnvalue_2 0.0)
        (bind _returnvalue_3 (`KismetMathLibrary.Conv_VectorToTransform` _output_get))
        (`InstancedStaticMeshComponent.AddInstance` (`self.Herbe`) _returnvalue_3)
        (else
          (`InstancedStaticMeshComponent.AddInstance` (`self.Terre`) _returnvalue_3)))
      (set `self.nombreIterration` 3))))

(fn `UserConstructionScript`)