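; Player character for a block-building game, handling movement, jump, camera look, a 12-slot toolbar and block placement.
; BeginPlay creates the master HUD only for the locally controlled pawn; shortcut and next/previous inputs set a wrapping slot index and swap toolbar materials.
; The "Casser" (break) input actually places blocks: a camera line trace finds BP_Terrain_Generation, then S_ and M_PlacerBloc events relay impact point and slot index to its Placer.
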(event `InputAction|Raccourci1`
  (params (Key :type "Key Structure"))
  (bind _bpw_toolbar (`/Game/SurvivalTime/UI/BPW__MasterHUD.BPW_Toolbar` (`self.MasterHUD`)))
  ;[1 1 1] Gestion raccourci clavier
  (:`Pressed`
    (set `self.selectToolbar` 0)
    ;[1 1 1] Reset des case qui ne sont ppas séléctionner
    (`Image.SetBrushFromMaterial` (`/Game/SurvivalTime/UI/BPW_Toolbar.T1` (`/Game/SurvivalTime/UI/BPW__MasterHUD.BPW_Toolbar` (`self.MasterHUD`))) "/Game/SurvivalTime/MaterielLibrary/UI/M_Toolbar.M_Toolbar" :!label _label)
    (`Image.SetBrushFromMaterial` (`/Game/SurvivalTime/UI/BPW_Toolbar.T2` (`/Game/SurvivalTime/UI/BPW__MasterHUD.BPW_Toolbar` (`self.MasterHUD`))) "/Game/SurvivalTime/MaterielLibrary/UI/M_Toolbar.M_Toolbar")
    (`Image.SetBrushFromMaterial` (`/Game/SurvivalTime/UI/BPW_Toolbar.T3` (`/Game/SurvivalTime/UI/BPW__MasterHUD.BPW_Toolbar` (`self.MasterHUD`))) "/Game/SurvivalTime/MaterielLibrary/UI/M_Toolbar.M_Toolbar")
    (`Image.SetBrushFromMaterial` (`/Game/SurvivalTime/UI/BPW_Toolbar.T4` (`/Game/SurvivalTime/UI/BPW__MasterHUD.BPW_Toolbar` (`self.MasterHUD`))) "/Game/SurvivalTime/MaterielLibrary/UI/M_Toolbar.M_Toolbar")
    (`Image.SetBrushFromMaterial` (`/Game/SurvivalTime/UI/BPW_Toolbar.T5` (`/Game/SurvivalTime/UI/BPW__MasterHUD.BPW_Toolbar` (`self.MasterHUD`))) "/Game/SurvivalTime/MaterielLibrary/UI/M_Toolbar.M_Toolbar")
    (`Image.SetBrushFromMaterial` (`/Game/SurvivalTime/UI/BPW_Toolbar.T6` (`/Game/SurvivalTime/UI/BPW__MasterHUD.BPW_Toolbar` (`self.MasterHUD`))) "/Game/SurvivalTime/MaterielLibrary/UI/M_Toolbar.M_Toolbar")
    (`Image.SetBrushFromMaterial` (`/Game/SurvivalTime/UI/BPW_Toolbar.T7` (`/Game/SurvivalTime/UI/BPW__MasterHUD.BPW_Toolbar` (`self.MasterHUD`))) "/Game/SurvivalTime/MaterielLibrary/UI/M_Toolbar.M_Toolbar")
    (`Image.SetBrushFromMaterial` (`/Game/SurvivalTime/UI/BPW_Toolbar.T8` (`/Game/SurvivalTime/UI/BPW__MasterHUD.BPW_Toolbar` (`self.MasterHUD`))) "/Game/SurvivalTime/MaterielLibrary/UI/M_Toolbar.M_Toolbar")
    (`Image.SetBrushFromMaterial` (`/Game/SurvivalTime/UI/BPW_Toolbar.T9` (`/Game/SurvivalTime/UI/BPW__MasterHUD.BPW_Toolbar` (`self.MasterHUD`))) "/Game/SurvivalTime/MaterielLibrary/UI/M_Toolbar.M_Toolbar")
    (`Image.SetBrushFromMaterial` (`/Game/SurvivalTime/UI/BPW_Toolbar.T11` (`/Game/SurvivalTime/UI/BPW__MasterHUD.BPW_Toolbar` (`self.MasterHUD`))) "/Game/SurvivalTime/MaterielLibrary/UI/M_Toolbar.M_Toolbar")
    (`Image.SetBrushFromMaterial` (`/Game/SurvivalTime/UI/BPW_Toolbar.T10` (`/Game/SurvivalTime/UI/BPW__MasterHUD.BPW_Toolbar` (`self.MasterHUD`))) "/Game/SurvivalTime/MaterielLibrary/UI/M_Toolbar.M_Toolbar")
    (`Image.SetBrushFromMaterial` (`/Game/SurvivalTime/UI/BPW_Toolbar.T12` (`/Game/SurvivalTime/UI/BPW__MasterHUD.BPW_Toolbar` (`self.MasterHUD`))) "/Game/SurvivalTime/MaterielLibrary/UI/M_Toolbar.M_Toolbar")
    ;[1 1 1] Séléction dans la toolbar
    (`Image.SetBrushFromMaterial` (select `int` (`self.selectToolbar`) :`0` (`/Game/SurvivalTime/UI/BPW_Toolbar.T1` _bpw_toolbar) :`1` (`/Game/SurvivalTime/UI/BPW_Toolbar.T2` _bpw_toolbar) :`2` (`/Game/SurvivalTime/UI/BPW_Toolbar.T3` _bpw_toolbar) :`3` (`/Game/SurvivalTime/UI/BPW_Toolbar.T4` _bpw_toolbar) :`4` (`/Game/SurvivalTime/UI/BPW_Toolbar.T5` _bpw_toolbar) :`5` (`/Game/SurvivalTime/UI/BPW_Toolbar.T6` _bpw_toolbar) :`6` (`/Game/SurvivalTime/UI/BPW_Toolbar.T7` _bpw_toolbar) :`7` (`/Game/SurvivalTime/UI/BPW_Toolbar.T8` _bpw_toolbar) :`8` (`/Game/SurvivalTime/UI/BPW_Toolbar.T9` _bpw_toolbar) :`9` (`/Game/SurvivalTime/UI/BPW_Toolbar.T10` _bpw_toolbar) :`10` (`/Game/SurvivalTime/UI/BPW_Toolbar.T11` _bpw_toolbar) :`11` (`/Game/SurvivalTime/UI/BPW_Toolbar.T12` _bpw_toolbar)) "/Game/SurvivalTime/MaterielLibrary/UI/M_Toolbar_Select.M_Toolbar_Select")))

(event `self.ReceiveBeginPlay`
  ;[1 1 1] Vérification que le BegginPlay ne concerne que l'instance bp_characctere du client, afin d'instancier qu'une seule toolbar
  (if (== (`Controller.K2_GetPawn` (`GameplayStatics.GetPlayerController` 0)) self)
    (bind _returnvalue (`|CreateWidget` "/Game/SurvivalTime/UI/BPW__MasterHUD.BPW__MasterHUD_C"))
    (bind _output_get (set `self.MasterHUD` _returnvalue))
    (`UserWidget.AddToViewport` _output_get 0)
    (`Image.SetBrushFromMaterial` (`/Game/SurvivalTime/UI/BPW_Toolbar.T1` (`/Game/SurvivalTime/UI/BPW__MasterHUD.BPW_Toolbar` (`self.MasterHUD`))) "/Game/SurvivalTime/MaterielLibrary/UI/M_Toolbar_Select.M_Toolbar_Select")))

(event `InputAction|Raccourci2`
  (params (Key :type "Key Structure"))
  ;[1 1 1] Gestion raccourci clavier
  (:`Pressed`
    (set `self.selectToolbar` 1)
    (goto _label)))

(event `InputAction|Raccourci3`
  (params (Key :type "Key Structure"))
  ;[1 1 1] Gestion raccourci clavier
  (:`Pressed`
    (set `self.selectToolbar` 2)
    (goto _label)))

(event `InputAction|Raccourci4`
  (params (Key :type "Key Structure"))
  ;[1 1 1] Gestion raccourci clavier
  (:`Pressed`
    (set `self.selectToolbar` 3)
    (goto _label)))

(event `InputAction|Raccourci5`
  (params (Key :type "Key Structure"))
  ;[1 1 1] Gestion raccourci clavier
  (:`Pressed`
    (set `self.selectToolbar` 4)
    (goto _label)))

(event `InputAction|Raccourci6`
  (params (Key :type "Key Structure"))
  ;[1 1 1] Gestion raccourci clavier
  (:`Pressed`
    (set `self.selectToolbar` 5)
    (goto _label)))

(event `InputAction|Raccourci7`
  (params (Key :type "Key Structure"))
  ;[1 1 1] Gestion raccourci clavier
  (:`Pressed`
    (set `self.selectToolbar` 6)
    (goto _label)))

(event `InputAction|Raccourci8`
  (params (Key :type "Key Structure"))
  ;[1 1 1] Gestion raccourci clavier
  (:`Pressed`
    (set `self.selectToolbar` 7)
    (goto _label)))

(event `InputAction|Raccourci9`
  (params (Key :type "Key Structure"))
  ;[1 1 1] Gestion raccourci clavier
  (:`Pressed`
    (set `self.selectToolbar` 8)
    (goto _label)))

(event `InputAxis|Vertical`
  (params (AxisValue :type "Float (single-precision)"))
  ;[1 1 1] Déplaement
  ;;[1 1 1] Déplacement sur avant / arriere
  (`self.AddMovementInput` (`self.GetActorForwardVector`) AxisValue))

(event `InputAction|Jump`
  (params (Key :type "Key Structure"))
  ;[1 1 1] Déplaement
  ;;[1 1 1] Saut
  (:`Pressed`
    (`self.Jump`)))

(event `InputAction|Raccourci0`
  (params (Key :type "Key Structure"))
  ;[1 1 1] Gestion raccourci clavier
  (:`Pressed`
    (set `self.selectToolbar` 9)
    (goto _label)))

(event `InputAction|Raccourci°`
  (params (Key :type "Key Structure"))
  ;[1 1 1] Gestion raccourci clavier
  (:`Pressed`
    (set `self.selectToolbar` 10)
    (goto _label)))

(event `InputAxis|Horizontal`
  (params (AxisValue :type "Float (single-precision)"))
  ;[1 1 1] Déplaement
  ;;[1 1 1] Déplacement droite gauche
  (`self.AddMovementInput` (`self.GetActorRightVector`) AxisValue))

(event `InputAction|Raccourci+`
  (params (Key :type "Key Structure"))
  ;[1 1 1] Gestion raccourci clavier
  (:`Pressed`
    (set `self.selectToolbar` 11)
    (goto _label)))

(event `InputAction|SelectRaccourciSuivant`
  (params (Key :type "Key Structure"))
  (bind _returnvalue (+ (`self.selectToolbar`) 1))
  ;[1 1 1] Selection de la toolbox de 0 vers 11
  (:`Pressed`
    (if (> _returnvalue 11)
      (set `self.selectToolbar` 0)
      (goto _label)
      (else
        (set `self.selectToolbar` _returnvalue)
        (goto _label)))))

(event `InputAxis|Turn`
  (params (AxisValue :type "Float (single-precision)"))
  ;[1 1 1] Rotation personnage
  (`self.AddControllerYawInput` AxisValue))

(event `InputAxis|LookUp`
  (params (AxisValue :type "Float (single-precision)"))
  ;[1 1 1] Rotation camera
  (`self.AddControllerPitchInput` AxisValue))

(event `InputAction|Casser`
  (params (Key :type "Key Structure"))
  (bind _camera (`self.Camera`))
  (bind _returnvalue (`SceneComponent.K2_GetComponentLocation` _camera))
  ;[1 1 1] Plaçage de bloc
  (:`Pressed`
    (bind _outhit (`KismetSystemLibrary.LineTraceSingle` _returnvalue (+ _returnvalue (* (`SceneComponent.GetForwardVector` _camera) 1000.0)) "TraceTypeQuery1"))
    (bind (_bblockinghit _binitialoverlap _time _distance _location _impactpoint _normal _impactnormal _physmat _hitactor) (`GameplayStatics.BreakHitResult` _outhit))
    (bind _asbp_terrain_generation (cast `/Game/SurvivalTime/Blueprint/World/BP_Terrain_Generation` _hitactor))
    (`self.S_PlacerBloc` _asbp_terrain_generation _impactpoint (`self.selectToolbar`))))

(event `InputAction|SelectRaccourciPrecedent`
  (params (Key :type "Key Structure"))
  (bind _returnvalue (+ (`self.selectToolbar`) -1))
  ;[1 1 1] Selection de la toolbox de 11 vers 0
  (:`Pressed`
    (if (< _returnvalue 0)
      (set `self.selectToolbar` 11)
      (goto _label)
      (else
        (set `self.selectToolbar` _returnvalue)
        (goto _label)))))

(event `S_PlacerBloc`
  (params (Map :type "/Game/SurvivalTime/Blueprint/World/BP_Terrain_Generation Object Reference") (Position :type "Vector Structure") (`Id Bloc` :type Integer))
  ;[1 1 1] Plaçage de bloc
  (`self.M_PlacerBloc` Position Map `Id Bloc`))

(event `M_PlacerBloc`
  (params (Position :type "Vector Structure") (Map :type "/Game/SurvivalTime/Blueprint/World/BP_Terrain_Generation Object Reference") (idBloc :type Integer))
  ;[1 1 1] Plaçage de bloc
  (`/Game/SurvivalTime/Blueprint/World/BP_Terrain_Generation.Placer` Map Position idBloc))

(fn `UserConstructionScript`)